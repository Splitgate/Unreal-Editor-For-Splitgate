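; Map helper Blueprint that, judging by its name, keeps weapon content always loaded by holding references to it in an ObjectsToLoad array.
; The Food function recursively queries the Asset Registry for everything under /Game/Weapons and resolves each result with GetAsset.
; Add Asset appends each object only if the array does not already contain it.
; The construction script is empty, and nothing in this Blueprint calls Food.
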(fn ConstructionScript)

(fn Food
  (bind _outassetdata (Class|AssetRegistry|GetAssetsbyPath (Class|AssetRegistryHelpers|GetAssetRegistry) "/Game/Weapons" true false))
  (for _array_element _outassetdata
    (Utilities|AddAsset (Class|AssetRegistryHelpers|GetAsset _array_element))))