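; BP_BaseCustomGameMode is a base custom game mode that can periodically clear pickups from the world.
; On BeginPlay, if AutoClearPickups is enabled, it starts a looping timer at ClearInterval.
; Each tick of the timer destroys every ARPickup_BP actor, calling Say with the total count inside the loop, so the message repeats once per pickup.
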(event EventBeginPlay
  (Utilities|FlowControl|Sequence
    (:then_0
      (|AutoClearPickups))))

(fn ConstructionScript
  (|CallParentFunction))

(event Custom|OnClearPickup
  (bind _outactors (Actor|GetAllActorsOfClass "/Game/Pickups/DroppedGunPickups/ARPickup_BP.ARPickup_BP_C"))
  (for _array_element _outactors
    (Actor|DestroyActor _array_element)
    (Class|GameMode|Say (Utilities|String|ToString(Text) (Utilities|Text|FormatText "Cleared {%s} Pickups!" (Utilities|Array|Length _outactors))))))