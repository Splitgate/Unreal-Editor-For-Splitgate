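; Chaos game mode that scrambles portal links and randomly flings players, driven by two looping timers started on BeginPlay.
; A fast timer shuffles all portals and links them in a ring, occasionally spawning a random gun at the last linked portal when wormhole portals are enabled.
; A slower timer launches a random character with added vertical velocity, though each velocity component comes from a separate random pick.
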(event Custom|:Fling
  (bind _outactors (Actor|GetAllActorsOfClass "/Script/PortalWars.PortalWarsCharacter"))
  (bind _output_get (Variables|PlayerChaos|SetPlayers _outactors))
  (Utilities|Array|Shuffle _output_get)
  (PlayerChaos|ProcessPlayerArray (Variables|PlayerChaos|GetPlayers)))

(event Custom|RandomizePortals
  (bind _outactors (Actor|GetAllActorsOfClass "/Script/PortalWars.Portal"))
  (bind _output_get (Variables|PortalChaos|SetPortals _outactors))
  (Utilities|Array|Shuffle _output_get)
  (PortalChaos|ProcessPortalsArray (Variables|PortalChaos|GetPortals)))

(event EventBeginPlay
  (Utilities|Time|SetTimerbyEvent (delegate Custom|RandomizePortals) 0.5 true)
  (Utilities|Time|SetTimerbyEvent (delegate Custom|:Fling) 5.0 true))

(fn ConstructionScript
  (|CallParentFunction))

(fn ProcessPortalsArray
  (params (Array :type Array%20of%20Portal%20Object%20References))
  (bind _random_gun_array (Variables|PortalChaos|GetRandom%20Gun%20Array))
  (bind _output (Utilities|GetRandomArrayItem _random_gun_array))
  (for (_array_element _array_index) Array
    (bind _output_get (Variables|/Script/PortalWars.Portal|SetLinkedPortal (Utilities|Array|Get(acopy) Array (select (== (+ _array_index 1) (Utilities|Array|Length Array)) 0 (+ _array_index 1))) _array_element))
    (LocalVariables|SetLinked%20Portal%20Ref _output_get))
  (if (Variables|PortalChaos|GetUse%20Wormhole%20Portals)
    (if (>= (Math|Random|RandomIntegerinRange 0 25) 23)
      (if (Utilities|IsValidClass _output)
        (bind _returnvalue (Game|SpawnActorfromClass _output (Math|Transform|MakeTransform (+ (* (Transformation|GetActorForwardVector (LocalVariables|GetLinked%20Portal%20Ref)) 1.5e+02) (.location (Transformation|GetActorTransform (LocalVariables|GetLinked%20Portal%20Ref)))) (.rotation (Transformation|GetActorTransform (LocalVariables|GetLinked%20Portal%20Ref))) (.scale (Transformation|GetActorTransform (LocalVariables|GetLinked%20Portal%20Ref)))) "AdjustIfPossibleButAlwaysSpawn" 0 0))
        (if (== (Utilities|GetClass _returnvalue) "/Game/Pickups/DroppedGunPickups/InstaGib_RailGunPickup_BP.InstaGib_RailGunPickup_BP_C")
          _)))))

(fn ProcessPlayerArray
  (params (Array :type Array%20of%20Portal%20Wars%20Character%20Object%20References))
  (bind _output (Utilities|GetRandomArrayItem Array))
  (bind _returnvalue (Transformation|GetVelocity _output))
  (Character|LaunchCharacter _output (Math|Vector|MakeVector (.x _returnvalue) (.y _returnvalue) (+ (.z _returnvalue) (Variables|PlayerChaos|GetFling))) false true))