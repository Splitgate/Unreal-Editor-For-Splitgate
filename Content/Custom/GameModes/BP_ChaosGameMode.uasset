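; Chaos game mode that keeps rewiring the level's portal connections at random during play.
; A looping half-second timer started on BeginPlay gathers every Portal actor and shuffles the list.
; It then sets each portal's LinkedPortal to its predecessor in the shuffled order, wrapping around so all portals form a single one-way ring.
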(event Custom|RandomizePortals
  (bind _outactors (Actor|GetAllActorsOfClass "/Script/PortalWars.Portal"))
  (bind _output_get (Variables|Default|SetPortals _outactors))
  (Utilities|Array|Shuffle _output_get)
  (CallFunction|ProcessPortalsArray (Variables|Default|GetPortals)))

(event EventBeginPlay
  (Utilities|Time|SetTimerbyEvent (delegate Custom|RandomizePortals) 0.5 true))

(fn ConstructionScript
  (|CallParentFunction))

(fn ProcessPortalsArray
  (params (Array :type Array%20of%20Portal%20Object%20References))
  (for (_array_element _array_index) Array
    (Variables|/Script/PortalWars.Portal|SetLinkedPortal (Utilities|Array|Get(acopy) Array (select (== (+ _array_index 1) (Utilities|Array|Length Array)) 0 (+ _array_index 1))) _array_element)))