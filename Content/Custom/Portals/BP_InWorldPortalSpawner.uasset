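; BP_InWorldPortalSpawner is a placeable helper actor that creates a linked pair of portals in the level.
; On BeginPlay it spawns PortalClass at the transforms of its two marker components via SpawnPortal, always spawning regardless of collision.
; It then sets each portal as the other's LinkedPortal and destroys itself, leaving only the portals in the world.
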(event EventBeginPlay
  (Utilities|FlowControl|Sequence
    (:then_0
      ;[0 0.5572 1] spawn portals
      (Utilities|FlowControl|Sequence
        (:then_0
          (bind _returnvalue (CallFunction|SpawnPortal (Variables|Default|GetPortal1Marker)))
          (Variables|Default|SetPortal1 _returnvalue))
        (:then_1
          (bind _returnvalue_2 (CallFunction|SpawnPortal (Variables|Default|GetPortal2Marker)))
          (Variables|Default|SetPortal2 _returnvalue_2))))
    (:then_1
      ;[0.8968 0 1] set portal 2's linked portal to be portal 1
      (Variables|/Script/PortalWars.Portal|SetLinkedPortal (Variables|Default|GetPortal2) (Variables|Default|GetPortal1))
      ;[0.8968 0 1] set portal 1's linked portal to be portal 2
      (Variables|/Script/PortalWars.Portal|SetLinkedPortal (Variables|Default|GetPortal1) (Variables|Default|GetPortal2)))
    (:then_2
      ;[1 0.2055 0] destroy after portals spawned
      (Actor|DestroyActor))))

(fn ConstructionScript)

(fn SpawnPortal
  (params (Component :type Arrow%20Component%20Object%20Reference))
  (bind _returnvalue (Game|SpawnActorfromClass (Variables|Default|GetPortalClass) (Transformation|GetWorldTransform Component) "AlwaysSpawn" 0 0))
  (bind _asportal (Utilities|Casting|CastToPortal _returnvalue))
  (return _asportal))