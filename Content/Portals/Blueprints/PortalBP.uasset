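; PortalBP is a portal actor that takes on a left or right portal color.
; Its construction script creates a dynamic instance of the Portal_Fill material, sets its Emissive Color from IsLeftPortal, and applies it to the portal mesh.
; The event graph holds only disabled default events, so the Blueprint itself contains no teleport or overlap logic.
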(event EventBeginPlay)

(event Collision|EventActorBeginOverlap
  (params (OtherActor :type Actor%20Object%20Reference)))

(event EventTick
  (params (DeltaSeconds :type Float%20%28single-precision%29)))

(fn ConstructionScript
  (bind _returnvalue (Rendering|Material|CreateDynamicMaterialInstance "/Game/Portals/Materials/Portal_Fill.Portal_Fill" "None" :!class /Script/Engine.KismetMaterialLibrary))
  (LocalVariables|SetPortal%20Mat _returnvalue)
  (if (Variables|Default|GetIsLeftPortal)
    (Rendering|Material|SetVectorParameterValue (LocalVariables|GetPortal%20Mat) "Emissive Color" (Variables|Default|GetLeftPortalColor) :!class /Script/Engine.MaterialInstanceDynamic)
    (else
      (Rendering|Material|SetVectorParameterValue (LocalVariables|GetPortal%20Mat) "Emissive Color" (Variables|Default|GetRightPortalColor) :!class /Script/Engine.MaterialInstanceDynamic)))
  (Rendering|Material|SetMaterial (Variables|Default|GetPortal%20Mesh%20%28TEMP%20DO%20NOT%20MODIFY%20THIS%20CLASS%29) 0 (LocalVariables|GetPortal%20Mat)))